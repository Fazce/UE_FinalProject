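; BP_CharacterGlider is a player character Blueprint that glides while the special input is held in mid-air.
; Pressing IA_Special while falling sets IsGliding, sharply lowers gravity and raises air control.
; A zero-velocity LaunchCharacter with Z override cancels vertical speed as the glide starts, keeping horizontal momentum.
; Input completion clears the flag and sets gravity and air control back to fixed normal values, with no separate landing check.
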(event `EnhancedInput|/Game/Input/Actions/IA_Special`
  (params (ActionValue :type "Vector2D Structure") (ElapsedSeconds :type "Float (double-precision)") (TriggeredSeconds :type "Float (double-precision)") (InputAction :type "InputAction Object Reference" :default "/Game/Input/Actions/IA_Special.IA_Special"))
  (:`Started`
    (if (`NavMovementComponent.IsFalling` (`self.CharacterMovement`))
      (bind _output_get (set `self.isGliding` true))
      (`self.LaunchCharacter` (0.0 0.0 0.0) false _output_get)
      (set `CharacterMovementComponent.GravityScale` 0.05 (`self.CharacterMovement`))
      (set `CharacterMovementComponent.AirControl` 1.0 (`self.CharacterMovement`))))
  (:`Completed`
    (set `self.isGliding` false)
    (set `CharacterMovementComponent.GravityScale` 1.0 (`self.CharacterMovement`))
    (set `CharacterMovementComponent.AirControl` 0.35 (`self.CharacterMovement`))))

(fn `UserConstructionScript`
  (`parent.UserConstructionScript`))